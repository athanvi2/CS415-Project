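; BP_DiceGameCharacter is a dice game character Blueprint that holds HP and shows it on a health bar.
; ApplyDamage and ApplyHealing subtract or add an amount through SetHP, with no clamping.
; When the value changes, SetHP stores it and pushes it to the WBP_HealthBar inside its Widget component, assuming a maximum of 100.
; BeginPlay and the construction script are empty.
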(event EventBeginPlay)

(fn ConstructionScript)

(fn GetHP
  (return (Variables|Default|GetHP)))

(fn SetHP
  (params (HP :type Integer))
  (if (!= HP (Variables|Default|GetHP))
    (Variables|Default|SetHP HP)
    (Progress|SetPercent (Variables|/Game/Blueprints/UI/WBP_HealthBar.WBP_HealthBar_C|GetHealthBar (.AsWBP%20Health%20Bar (Utilities|Casting|CastToWBP_HealthBar (UserInterface|GetWidget (Variables|Default|GetWidget))))) (/ (Math|Conversions|ToFloat(Integer) (Variables|Default|GetHP)) 1e+02))))

(fn ApplyDamage
  (params (Amount :type Integer))
  (CallFunction|SetHP (- (Variables|Default|GetHP) Amount)))

(fn ApplyHealing
  (params (Amount :type Integer))
  (CallFunction|SetHP (+ Amount (Variables|Default|GetHP))))