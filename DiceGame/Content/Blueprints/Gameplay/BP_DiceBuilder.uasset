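; BP_DiceBuilder is a board of randomized dice faces from which six selected faces become a new die.
; The construction script lays out a centered grid of child actors, each randomly a damage or heal face, indexed with selection metadata.
; FaceClicked toggles a face's selection and its custom depth rendering.
; CreateDice gathers selected faces and spawns BP_Dice with them, or prints an error if the count is not six.
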(event Custom|FaceClicked
  (params (Face :type BP%20Dice%20Face%20Object%20Reference))
  (bind _dicefaceindex (Variables|Default|GetDiceFaceIndex))
  (bind _dicefacemeta (Variables|Default|GetDiceFaceMeta))
  (bind (_value _returnvalue) (Utilities|Map|Find _dicefaceindex Face))
  (bind _output (Utilities|Array|Get(acopy) _dicefacemeta _value))
  (Variables|Default|SetClickedFace Face)
  (if _returnvalue
    (if (.Selected (Utilities|Struct|BreakF_DiceFaceMeta _output))
      (Utilities|Struct|SetmembersinF_DiceFaceMeta _output false)
      (Rendering|SetRenderCustomDepth (Variables|/Game/Blueprints/Gameplay/BP_DiceFace.BP_DiceFace_C|GetPlane (Variables|Default|GetClickedFace)) false)
      (else
        (Utilities|Struct|SetmembersinF_DiceFaceMeta _output true)
        (Rendering|SetRenderCustomDepth (Variables|/Game/Blueprints/Gameplay/BP_DiceFace.BP_DiceFace_C|GetPlane (Variables|Default|GetClickedFace)) true)))))

(fn ConstructionScript
  (Utilities|FlowControl|Sequence
    (:then_0
      (Utilities|Array|Resize (Variables|Default|GetDiceFaceMeta) (* (Variables|Default|GetNumberOfRows) (Variables|Default|GetNumberOfColumns)))
      (for _index (range 0 (- (Variables|Default|GetNumberOfColumns) 1))
        (for _index_2 (range 0 (- (Variables|Default|GetNumberOfRows) 1))
          (CallFunction|CreateFaceatPosition _index _index_2))))
    (:then_1
      (Transformation|SetWorldTransform (Variables|Default|GetPostProcess) (Math|Transform|MakeTransform "0, 0, 0" "0, 0, 0" "1.000000,1.000000,1.000000") false false))))

(fn CreateFaceatPosition
  (params (Row :type Integer) (Column :type Integer))
  (bind _numberofcolumns (Variables|Default|GetNumberOfColumns))
  (bind _dicefacesize (Variables|Default|GetDiceFaceSize))
  (bind _dicefacesize_2 (Variables|Default|GetDiceFaceSize))
  (bind _dicefacesize_3 (Variables|Default|GetDiceFaceSize))
  (bind _returnvalue (/ _dicefacesize_2 2.0))
  (bind _returnvalue_2 (/ _dicefacesize 1e+02))
  (bind _returnvalue_3 (* Row _numberofcolumns))
  (bind _returnvalue_4 (+ _returnvalue_3 Column))
  (bind _returnvalue_5 (AddComponent|AddChildActorComponent false (Math|Transform|MakeTransform (Math|Vector|MakeVector (- (* Row _dicefacesize_3) (- (/ (* (Variables|Default|GetNumberOfRows) (Variables|Default|GetDiceFaceSize)) 2) _returnvalue)) (- (* Column _dicefacesize_3) (- (/ (* (Variables|Default|GetNumberOfColumns) (Variables|Default|GetDiceFaceSize)) 2) _returnvalue)) 0.0) "0, 0, 0" (Math|Vector|MakeVector _returnvalue_2 _returnvalue_2 1.0))))
  (ChildActorComponent|SetChildActorClass _returnvalue_5 (Utilities|Select :Index (Math|Random|RandomInteger 2) :Option%200 "/Game/Blueprints/Gameplay/DiceFaces/BP_DiceFaceDamage.BP_DiceFaceDamage_C" :Option%201 "/Game/Blueprints/Gameplay/DiceFaces/BP_DiceFaceHeal.BP_DiceFaceHeal_C"))
  (bind _output_get (LocalVariables|SetFace (.AsBP%20Dice%20Face (Utilities|Casting|CastToBP_DiceFace (Variables|/Script/Engine.ChildActorComponent|GetChildActor _returnvalue_5)))))
  (Default|Randomize _output_get 1 10)
  (Utilities|Map|Add (Variables|Default|GetDiceFaceIndex) (LocalVariables|GetFace) _returnvalue_4)
  (Utilities|Array|SetArrayElem (Variables|Default|GetDiceFaceMeta) _returnvalue_4 (Utilities|Struct|MakeF_DiceFaceMeta (LocalVariables|GetFace) Row Column false)))

(fn CreateDice
  (Utilities|FlowControl|Sequence
    (:then_0
      (for _array_element (Variables|Default|GetDiceFaceMeta)
        (if (.selected _array_element)
          (Utilities|Array|Add (LocalVariables|GetDiceFaces) (.face _array_element)))))
    (:then_1
      (if (!= (Utilities|Array|Length (LocalVariables|GetDiceFaces)) 6)
        (Development|PrintString "Incorret number of faces")
        (else
          (bind _returnvalue (Game|SpawnActorfromClass "/Game/Blueprints/Gameplay/BP_Dice.BP_Dice_C" (Math|Transform|MakeTransform "0.000000,0.000000,9999.000000" "0, 0, 0" "1.000000,1.000000,1.000000") "Undefined" "MultiplyWithRoot" 0 (LocalVariables|GetDiceFaces) 0))
          (return _returnvalue))))))