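; Game mode for a dice combat game that owns the player character, dice builder and debug menu.
; BeginPlay adds the menu and spawns the player parked high above the level until StartCombat places it opposite the enemies at mirrored positions.
; The dice builder spawns on first show and hides by moving far overhead instead of being destroyed.
; ProcessActions prints each combat action, then applies damage or healing to its target.
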(event EventBeginPlay
  (Utilities|FlowControl|Sequence
    (:then_0
      (bind _returnvalue (UserInterface|CreateWidget "/Game/Blueprints/UI/WBP_DebugMenu.WBP_DebugMenu_C"))
      (bind _output_get (Variables|Default|SetDebugMenu _returnvalue))
      (UserInterface|Viewport|AddtoViewport _output_get 0))
    (:then_1
      (CallFunction|CreatePlayerCharacter))))

(fn ConstructionScript)

(fn StartCombat
  (params (Enemy :type Array%20of%20BP%20Dice%20Game%20Character%20Enemy%20Object%20References))
  (Utilities|FlowControl|Sequence
    (:then_0
      (Utilities|IsValid (Variables|Default|GetPlayer)
        (:Is%20Valid
          (Transformation|SetActorLocation (Variables|Default|GetPlayer) (Variables|Default|GetPlayerStartLocation) false false))
        (:Is%20Not%20Valid
          (CallFunction|CreatePlayerCharacter)
          (Transformation|SetActorLocation (Variables|Default|GetPlayer) (Variables|Default|GetPlayerStartLocation) false false))))
    (:then_1
      (for _array_element Enemy
        (Transformation|SetActorLocation _array_element (* (Variables|Default|GetPlayerStartLocation) -1.0) false false)))))

(fn CreatePlayerCharacter
  (bind _playerstarttransform (Variables|Default|GetPlayerStartTransform))
  (bind _returnvalue (Game|SpawnActorfromClass "/Game/Blueprints/Gameplay/BP_DiceGameCharacterPlayer.BP_DiceGameCharacterPlayer_C" (Math|Transform|MakeTransform (Math|Vector|MakeVector (.x (.location _playerstarttransform)) (.y (.location _playerstarttransform)) 9999.0) (.rotation _playerstarttransform) (.scale _playerstarttransform)) "Undefined" "MultiplyWithRoot" 0 0))
  (Variables|Default|SetPlayer _returnvalue))

(fn ShowDiceBuilder
  (Utilities|IsValid (Variables|Default|GetDiceBuilder)
    (:Is%20Valid
      (Transformation|SetWorldTransform (Variables|/Script/Engine.Actor|GetRootComponent (Variables|Default|GetDiceBuilder)) (Math|Transform|MakeTransform "0, 0, 0" "0.000000,180.000000,0.000000" "1.000000,1.000000,1.000000") false false))
    (:Is%20Not%20Valid
      (bind _returnvalue (Game|SpawnActorfromClass "/Game/Blueprints/Gameplay/BP_DiceBuilder.BP_DiceBuilder_C" (Math|Transform|MakeTransform "0, 0, 0" "0.000000,180.000000,0.000000" "1.000000,1.000000,1.000000") "Undefined" "MultiplyWithRoot" 0 4 4 0))
      (Variables|Default|SetDiceBuilder _returnvalue))))

(fn HideDiceBuilder
  (Utilities|IsValid (Variables|Default|GetDiceBuilder)
    (:Is%20Valid
      (Transformation|SetWorldTransform (Variables|/Script/Engine.Actor|GetRootComponent (Variables|Default|GetDiceBuilder)) (Math|Transform|MakeTransform "0.000000,0.000000,9999.000000" "0.000000,90.000000,0.000000" "1.000000,1.000000,1.000000") false false))))

(fn GetPlayerCharacter
  (return (Variables|Default|GetPlayer)))

(fn ProcessActions
  (params (Actions :type Array%20of%20F%20Action%20Structures))
  (for _array_element Actions
    (Development|PrintText (Utilities|Text|FormatText "type: {type}, value: {value}, target: {target}" (Utilities|String|EnumtoString (.type _array_element)) (.value _array_element) (.targetcharacter _array_element)))
    (switch Utilities|FlowControl|Switch|SwitchonE_ActionType (.type _array_element)
      (:NewEnumerator0
        (Default|ApplyDamage (.targetcharacter _array_element) (.value _array_element)))
      (:NewEnumerator1
        (Default|ApplyHealing (.targetcharacter _array_element) (.value _array_element))))))