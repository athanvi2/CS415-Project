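; BP_DiceFaceDamage is a dice face that represents a damage amount.
; On BeginPlay it shows Amount in red on its WBP_Text widget.
; GetAction returns a single FAction carrying Amount, the parent BP_Dice as source, and the given source and target characters.
; Randomize rolls Amount as an integer within a given range, without refreshing the displayed text.
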(event EventBeginPlay
  (Variables|/Script/UMG.TextBlock|SetText (Variables|/Game/Blueprints/UI/WBP_Text.WBP_Text_C|GetText (.AsWBP%20Text (Utilities|Casting|CastToWBP_Text (UserInterface|GetWidget (Variables|Default|GetWidget))))) (Utilities|Text|ToText(Integer) (Variables|Default|GetAmount)))
  (Appearance|SetColorandOpacity (Variables|/Game/Blueprints/UI/WBP_Text.WBP_Text_C|GetText (.AsWBP%20Text (Utilities|Casting|CastToWBP_Text (UserInterface|GetWidget (Variables|Default|GetWidget))))) (Utilities|Struct|MakeSlateColor "(R=1.000000,G=0.000000,B=0.001610,A=1.000000)" "UseColor_Specified") :!class /Script/UMG.TextBlock))

(fn ConstructionScript)

(fn GetAction
  (params (From :type BP%20Dice%20Game%20Character%20Object%20Reference) (To :type BP%20Dice%20Game%20Character%20Object%20Reference))
  (return (Utilities|Array|MakeArray (Utilities|Struct|MakeF_Action "NewEnumerator0" (Variables|Default|GetAmount) (.AsBP%20Dice (Utilities|Casting|CastToBP_Dice (Actor|GetAttachParentActor self))) From To))))

(fn Randomize
  (params (Min :type Integer) (Max :type Integer))
  (Variables|Default|SetAmount (Math|Random|RandomIntegerinRange Min Max)))