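; Pawn for a dice game that lets the player click dice faces with the mouse.
; On left mouse press, it deprojects the cursor and line traces on the Visibility channel to find a BP_DiceFace.
; It then casts the face's attach parent to BP_DiceBuilder, stores both references, and passes the clicked face to the builder's FaceClicked.
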(event Input|MouseEvents|LeftMouseButton
  (params (Key :type Key%20Structure :default "None"))
  (:Pressed
    (bind _outhit (CallFunction|TraceMouse))
    (bind _asbp_dice_face (Utilities|Casting|CastToBP_DiceFace (.HitActor (Collision|BreakHitResult _outhit))))
    (bind _output_get (Variables|Default|SetDiceFace _asbp_dice_face))
    (bind _asbp_dice_builder (Utilities|Casting|CastToBP_DiceBuilder (Actor|GetAttachParentActor _output_get)))
    (bind _output_get_2 (Variables|Default|SetDiceBuilder _asbp_dice_builder))
    (Default|FaceClicked _output_get_2 (Variables|Default|GetDiceFace))))

(fn ConstructionScript)

(fn TraceMouse
  (bind _returnvalue (Game|GetPlayerController 0))
  (bind (_worldlocation _worlddirection) (Game|Player|ConvertMouseLocationToWorldSpace _returnvalue))
  (bind (_outhit _returnvalue_2) (Collision|LineTraceByChannel _worldlocation (+ _worldlocation (* _worlddirection 1e+04)) "TraceTypeQuery1" false 0 "None"))
  (return _outhit _returnvalue_2))